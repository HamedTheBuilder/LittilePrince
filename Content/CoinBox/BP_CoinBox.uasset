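; BP_CoinBox is a breakable box that releases coins when hit by an attacking BP_Prince.
; Each Tick while unbroken, it polls overlapping BP_Prince actors and checks the first one's IsAttacking flag instead of using overlap events.
; BreakBox sets Broken, hides the actor, disables collision, spawns a batch of BP_Coin at its location and sets a short lifespan to remove itself.
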(event `self.ReceiveTick`
  (params (DeltaSeconds :type "Float (single-precision)"))
  (bind _overlappingactors (`self.GetOverlappingActors` self "/Game/ThirdPerson/Blueprints/BP_Prince.BP_Prince_C"))
  (if (not (`self.bBroken`))
    (if (> (`KismetArrayLibrary.Array_Length` _overlappingactors) 0)
      (bind _asbp_third_person_character (cast `/Game/ThirdPerson/Blueprints/BP_Prince` (`|GetArrayItem` _overlappingactors)))
      (if (`/Game/ThirdPerson/Blueprints/BP_Prince.IsAttacking` _asbp_third_person_character)
        (`self.BreakBox`)))))

(fn `BreakBox`
  (set `self.bBroken` true)
  (`self.SetActorHiddenInGame` self true)
  (`self.SetActorEnableCollision` self false)
  (for _ (range 6)
    (`|SpawnActorFromClass` "/Game/CoinBox/BP_Coin.BP_Coin_C" (`KismetMathLibrary.MakeTransform` (`self.K2_GetActorLocation` self)) "AlwaysSpawn" "MultiplyWithRoot" null null))
  (`self.SetLifeSpan` 0.1))

(fn `UserConstructionScript`)