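; Actor component that keeps its owner hidden and without collision until the collected coin count reaches RequiredCoins.
; On BeginPlay it binds to the count-changed event on BP_CollectibleGameInstance and reveals immediately if the count already qualifies.
; Reveal restores visibility and collision, then calls UnbindAll on that shared event, which also removes every other listener's binding.
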(event `self.ReceiveBeginPlay`
  (bind _returnvalue (`self.GetOwner`))
  (`Actor.SetActorHiddenInGame` _returnvalue true)
  (`Actor.SetActorEnableCollision` _returnvalue false)
  (bind _asbp_collectible_game_instance (cast `/Game/Collectibles/BP_CollectibleGameInstance` (`GameplayStatics.GetGameInstance`)))
  (set `self.GI` _asbp_collectible_game_instance)
  (add `/Game/Collectibles/BP_CollectibleGameInstance.OnCollectedCountChanged` (`self.GI`) (`|CreateDelegate` :!event `HandleCoinsChanged`))
  (if (>= (`/Game/Collectibles/BP_CollectibleGameInstance.CollectedCount` (`self.GI`)) (`self.RequiredCoins`))
    (`self.Reveal`)))

(fn `HandleCoinsChanged`
  (params (NewCount :type Integer))
  (if (and (not (`self.bRevealed`)) (>= NewCount (`self.RequiredCoins`)))
    (`self.Reveal`)))

(fn `Reveal`
  (bind _returnvalue (`self.GetOwner`))
  (set `self.bRevealed` true)
  (`Actor.SetActorHiddenInGame` _returnvalue false)
  (`Actor.SetActorEnableCollision` _returnvalue true)
  (clear `/Game/Collectibles/BP_CollectibleGameInstance.OnCollectedCountChanged` (`self.GI`)))