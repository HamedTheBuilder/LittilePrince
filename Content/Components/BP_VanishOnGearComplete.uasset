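; BP_VanishOnGearComplete is a component that removes its owning actor once all gear pieces are collected.
; On BeginPlay it binds to the collectible GameInstance's all-pieces-collected event and also checks the current piece count, vanishing immediately if the set is already complete.
; Vanish hides the owner, disables its collision and sets a short lifespan so it is destroyed shortly after.
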(event `self.ReceiveBeginPlay`
  (bind _asbp_collectible_game_instance (cast `/Game/Collectibles/BP_CollectibleGameInstance` (`GameplayStatics.GetGameInstance`)))
  (set `self.GI` _asbp_collectible_game_instance)
  (add `/Game/Collectibles/BP_CollectibleGameInstance.OnAllGearPiecesCollected` (`self.GI`) (`|CreateDelegate` :!event `HandleGearComplete`))
  (if (>= (`/Game/Collectibles/BP_CollectibleGameInstance.GearPiecesCollected` (`self.GI`)) 3)
    (`self.Vanish`)))

(fn `HandleGearComplete`
  (`self.Vanish`))

(fn `Vanish`
  (bind _returnvalue (`self.GetOwner`))
  (`Actor.SetActorHiddenInGame` _returnvalue true)
  (`Actor.SetActorEnableCollision` _returnvalue false)
  (`Actor.SetLifeSpan` _returnvalue 0.75))