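; BP_TemporaryDisappear is a component that makes its owning actor vanish for a while after a player touches it, then brings it back.
; OnPlayerTouched starts a delay timer, and a CountdownActive flag ignores repeat touches until the cycle finishes.
; DoDisappear hides the owner and disables its collision, then a second timer calls DoReappear to restore both and re-arm the trigger.
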(fn `DoDisappear`
  (bind _returnvalue (`self.GetOwner`))
  (`Actor.SetActorHiddenInGame` _returnvalue true)
  (`Actor.SetActorEnableCollision` _returnvalue false)
  (`KismetSystemLibrary.K2_SetTimer` self "DoReappear" (`self.HiddenDuration`)))

(fn `DoReappear`
  (bind _returnvalue (`self.GetOwner`))
  (`Actor.SetActorHiddenInGame` _returnvalue false)
  (`Actor.SetActorEnableCollision` _returnvalue true)
  (set `self.bCountdownActive` false))

(fn `OnPlayerTouched`
  (if (not (`self.bCountdownActive`))
    (set `self.bCountdownActive` true)
    (`KismetSystemLibrary.K2_SetTimer` self "DoDisappear" (`self.DelayBeforeDisappear`))))