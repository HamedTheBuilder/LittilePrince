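; BP_FloatingMovement is an actor component that makes its owner hover, spinning it around the vertical axis while bobbing it up and down.
; BeginPlay stores the owner's starting location and optionally picks a random phase so instances do not move in sync.
; Each Tick adds a yaw rotation and sets the location from that stored origin plus a sine offset over accumulated time, without sweeping.
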(event `self.ReceiveBeginPlay`
  (set `self.InitialLocation` (`Actor.K2_GetActorLocation` (`self.GetOwner` self)))
  (set `self.PhaseOffset` (`KismetMathLibrary.SelectFloat` (`KismetMathLibrary.RandomFloatInRange` 0.0 6.2831853) 0.0 (`self.RandomizeStartOffset`))))

(event `self.ReceiveTick`
  (params (DeltaSeconds :type "Float (single-precision)"))
  (bind _returnvalue (`self.GetOwner` self))
  (`Actor.K2_AddActorWorldRotation` _returnvalue (`KismetMathLibrary.MakeRotator` 0.0 0.0 (* (`self.RotationSpeed`) DeltaSeconds)) false false)
  (bind _output_get (set `self.ElapsedTime` (+ (`self.ElapsedTime`) DeltaSeconds)))
  (`Actor.K2_SetActorLocation` _returnvalue (+ (`self.InitialLocation`) (`KismetMathLibrary.MakeVector` 0.0 0.0 (* (`KismetMathLibrary.Sin` (+ (* (* _output_get (`self.BobSpeed`)) 6.2831853) (`self.PhaseOffset`))) (`self.BobHeight`)))) false false))