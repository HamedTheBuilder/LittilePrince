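; BP_GearPiece1 is a collectible gear piece pickup that the player collects by overlapping it.
; On first overlap by player pawn 0, it sets Collected, notifies GearPieceTracker and spawns a sparkle Niagara effect.
; It then hides itself, disables collision and uses a short life span to self-destroy.
; An unconnected copy of this chain remains in the graph with different visibility and life span settings, and never runs.
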(event `self.ReceiveActorBeginOverlap`
  (params (OtherActor :type "Actor Object Reference"))
  (if (and (== OtherActor (`GameplayStatics.GetPlayerPawn` 0)) (not (`self.bCollected`)))
    (set `self.bCollected` true)
    (`/Game/Components/BP_GearPieceTracker.OnCollected` (`self.GearPieceTracker`))
    (`NiagaraFunctionLibrary.SpawnSystemAtLocation` "/Game/Collectibles/NS_PickupSparkle.NS_PickupSparkle" (`self.K2_GetActorLocation` self))
    (`self.SetActorHiddenInGame` true)
    (`self.SetActorEnableCollision` false)
    (`self.SetLifeSpan` 0.5)))

(fn `UserConstructionScript`)