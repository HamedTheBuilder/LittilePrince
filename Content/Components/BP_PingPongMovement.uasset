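; Actor component that moves its owner smoothly back and forth between its starting location and a point MoveDistance along MoveDirection.
; BeginPlay caches the start location and applies the auto-start flag; StartMoving can also enable movement.
; While moving, Tick accumulates time and sets an absolute, unswept location using cosine easing, so MoveSpeed acts as average travel speed.
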(event `self.ReceiveBeginPlay`
  (set `self.InitialLocation` (`Actor.K2_GetActorLocation` (`self.GetOwner`)))
  (set `self.bIsMoving` (`self.StartMovingImmediately`)))

(event `self.ReceiveTick`
  (params (DeltaSeconds :type "Float (single-precision)"))
  (bind _movedistance (`self.MoveDistance`))
  (bind _returnvalue (+ (`self.ElapsedTime`) DeltaSeconds))
  (if (`self.bIsMoving`)
    (set `self.ElapsedTime` _returnvalue)
    (`Actor.K2_SetActorLocation` (`self.GetOwner`) (+ (`self.InitialLocation`) (* (`KismetMathLibrary.Normal` (`self.MoveDirection`)) (* _movedistance (* (- 1.0 (`KismetMathLibrary.Cos` (/ (* (* _returnvalue (`self.MoveSpeed`)) 3.14159265) _movedistance))) 0.5)))) false false)))

(fn `StartMoving`
  (set `self.bIsMoving` true))