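; Game instance Blueprint that tracks collectible progress: a general count, gear pieces capped at three, and whether the rose has been reached.
; Each function updates its state and calls event dispatchers, with the rose event guarded to fire once.
; Count broadcasts re-add one after storing the increment, so they report one above the stored value.
; The all-gears check does likewise, so it fires at both two and three stored pieces.
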(fn `AddCollectible`
  (bind _returnvalue (+ (`self.CollectedCount`) 1))
  (set `self.CollectedCount` _returnvalue)
  (`self.OnCollectedCountChanged` _returnvalue))

(fn `AddGearPiece`
  (bind _returnvalue (+ (`self.GearPiecesCollected`) 1))
  (if (< (`self.GearPiecesCollected`) 3)
    (set `self.GearPiecesCollected` _returnvalue)
    (`self.OnGearPiecesChanged` _returnvalue)
    (if (>= _returnvalue 3)
      (`self.OnAllGearPiecesCollected`))))

(fn `MarkRoseReached`
  (if (not (`self.bRoseReached`))
    (set `self.bRoseReached` true)
    (`self.OnRoseReached`)))