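; Collectible pickup actor that increases the collectible count and heals the player when touched.
; On sphere overlap with the player pawn, it calls AddCollectible on BP_CollectibleGameInstance, then heals BP_Prince by a fixed amount.
; It then spawns a pickup sparkle effect, hides itself, disables collision and expires via a short life span instead of immediate destruction.
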(event `self.CollisionSphere.OnComponentBeginOverlap`
  (params (OverlappedComponent :type "PrimitiveComponent Object Reference") (OtherActor :type "Actor Object Reference") (OtherComp :type "PrimitiveComponent Object Reference") (OtherBodyIndex :type Integer) (bFromSweep :type Boolean) (SweepResult :type "HitResult Structure (by ref)"))
  (if (== OtherActor (`GameplayStatics.GetPlayerPawn` 0))
    (bind _asbp_collectible_game_instance (cast `/Game/Collectibles/BP_CollectibleGameInstance` (`GameplayStatics.GetGameInstance`)))
    (`/Game/Collectibles/BP_CollectibleGameInstance.AddCollectible` _asbp_collectible_game_instance)
    (bind _asbp_prince (cast `/Game/ThirdPerson/Blueprints/BP_Prince` OtherActor))
    (`/Game/ThirdPerson/Blueprints/BP_Prince.HealPlayer` _asbp_prince 25.0)
    (`NiagaraFunctionLibrary.SpawnSystemAtLocation` "/Game/Collectibles/NS_PickupSparkle.NS_PickupSparkle" (`self.K2_GetActorLocation` self))
    (`self.SetActorHiddenInGame` true)
    (`self.SetActorEnableCollision` false)
    (`self.SetLifeSpan` 0.1)))

(fn `UserConstructionScript`)