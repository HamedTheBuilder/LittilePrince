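; BP_SequenceTrigger is a trigger volume that plays a reward Level Sequence once the player has gathered enough collectibles.
; On TriggerBox overlap by the player pawn, it reads CollectedCount from BP_CollectibleGameInstance and compares it to a hard-coded threshold of three.
; When met, it sets HasPlayed to block replays and creates a player for RewardSequence; otherwise it prints a keep-collecting message.
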(event `self.TriggerBox.OnComponentBeginOverlap`
  (params (OverlappedComponent :type "PrimitiveComponent Object Reference") (OtherActor :type "Actor Object Reference") (OtherComp :type "PrimitiveComponent Object Reference") (OtherBodyIndex :type Integer) (bFromSweep :type Boolean) (SweepResult :type "HitResult Structure (by ref)"))
  (if (and (== OtherActor (`GameplayStatics.GetPlayerPawn` 0)) (not (`self.bHasPlayed`)))
    (bind _asbp_collectible_game_instance (cast `/Game/Collectibles/BP_CollectibleGameInstance` (`GameplayStatics.GetGameInstance`)))
    (if (>= (`/Game/Collectibles/BP_CollectibleGameInstance.CollectedCount` _asbp_collectible_game_instance) 3)
      (set `self.bHasPlayed` true)
      (bind _outactor (`LevelSequencePlayer.CreateLevelSequencePlayer` (`self.RewardSequence`)))
      (`MovieSceneSequencePlayer.Play` (`LevelSequenceActor.SequencePlayer` _outactor))
      (else
        (`KismetSystemLibrary.PrintString` "Need 3 collectibles - keep collecting!")))))

(fn `UserConstructionScript`)