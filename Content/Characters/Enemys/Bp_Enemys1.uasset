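; Melee enemy character that chases the player on sight and attacks when the player comes within range.
; Pawn sensing triggers an AI MoveTo toward the player, while Tick yaws the enemy to face a player in melee range and starts attacks off cooldown.
; Each attack plays a montage, then after a fixed delay damages BP_Prince and launches it away with upward lift, without rechecking range at impact.
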(event `PerformMeleeAttack`
  (set `self.AttackOnCooldown` true)
  (set `self.IsAttacking` true)
  (`self.PlayAnimMontage` (`self.AttackMontage`))
  (`KismetSystemLibrary.Delay` 0.5)
  (`self.AttackHitNotify`)
  (`KismetSystemLibrary.Delay` 1.5)
  (set `self.AttackOnCooldown` false))

(event `self.ReceiveTick`
  (params (DeltaSeconds :type "Float (single-precision)"))
  (bind _returnvalue (`GameplayStatics.GetPlayerCharacter` 0))
  (bind _returnvalue_2 (`self.GetDistanceTo` _returnvalue))
  (if (and (> _returnvalue_2 1.0) (<= _returnvalue_2 (`self.MeleeRange`)))
    (`self.K2_SetActorRotation` (`KismetMathLibrary.MakeRotator` 0.0 0.0 (.yaw (`KismetMathLibrary.FindLookAtRotation` (`self.K2_GetActorLocation` self) (`self.K2_GetActorLocation` _returnvalue)))))
    (if (not (`self.AttackOnCooldown`))
      (`self.PerformMeleeAttack`))))

(event `AttackHitNotify`
  (bind _knockbackforce (`self.KnockbackForce`))
  (bind _asbp_prince (cast `/Game/ThirdPerson/Blueprints/BP_Prince` (`GameplayStatics.GetPlayerCharacter` 0)))
  (`/Game/ThirdPerson/Blueprints/BP_Prince.TakeDamage` _asbp_prince (`self.AttackDamage`))
  (bind _returnvalue (`KismetMathLibrary.Vector_Normal2D` (- (`self.K2_GetActorLocation` _asbp_prince) (`self.K2_GetActorLocation` self))))
  (`self.LaunchCharacter` _asbp_prince (`KismetMathLibrary.MakeVector` (* (.x _returnvalue) _knockbackforce) (* (.y _returnvalue) _knockbackforce) (`self.KnockbackLift`)) true true)
  (set `self.IsAttacking` false))

(event `ChasePlayer`
  (`|AIMoveTo` self (0.0 0.0 0.0) (`GameplayStatics.GetPlayerCharacter` 0) 120.0))

(event `self.PawnSensing.OnSeePawn`
  (params (Pawn :type "Pawn Object Reference"))
  (`self.ChasePlayer`))

(fn `UserConstructionScript`)